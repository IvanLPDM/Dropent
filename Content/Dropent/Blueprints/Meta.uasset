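; Meta is a goal actor that declares a win when the Ball enters its Sphere trigger.
; On BeginPlay it pre-creates the Win widget and, if a third-person character exists, stores that character's transform in RespawnPos, then overwrites it with the Ball's.
; A Ball overlap sets the Win flag, shows the widget, and after a short delay calls Restart on the character reference.
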(event OnComponentBeginOverlap(Sphere)
  (params (OverlappedComponent :type Primitive%20Component%20Object%20Reference) (OtherActor :type Actor%20Object%20Reference) (OtherComp :type Primitive%20Component%20Object%20Reference) (OtherBodyIndex :type Integer) (bFromSweep :type Boolean) (SweepResult :type Hit%20Result%20Structure%20%28by%20ref%29))
  (Utilities|Casting|CastToBall OtherActor)
  (Variables|Default|SetWin true)
  (UserInterface|Viewport|AddtoViewport (Variables|Default|GetWinWidget) 0)
  (Utilities|FlowControl|Delay 4.0)
  (Default|Restart (stale EventBeginPlay _returnvalue)))

(event EventBeginPlay
  (Utilities|FlowControl|Sequence
    (:then_0
      (bind _returnvalue (Actor|GetActorOfClass "/Game/ThirdPerson/Blueprints/BP_ThirdPersonCharacter.BP_ThirdPersonCharacter_C"))
      (if (Utilities|IsValid _returnvalue)
        (Utilities|FlowControl|Sequence
          (:then_0
            (Variables|Default|SetRespawnPos (Math|Transform|MakeTransform (.location (Transformation|GetActorTransform _returnvalue)) (.rotation (Transformation|GetActorTransform _returnvalue)) (.scale (Transformation|GetActorTransform _returnvalue)))))
          (:then_1
            (bind _returnvalue_2 (Actor|GetActorOfClass "/Game/Dropent/Blueprints/Ball.Ball_C"))
            (Variables|Default|SetRespawnPos (Math|Transform|MakeTransform (.location (Transformation|GetActorTransform _returnvalue_2)) (.rotation (Transformation|GetActorTransform _returnvalue_2)) (.scale (Transformation|GetActorTransform _returnvalue_2))))))))
    (:then_1
      (bind _returnvalue_3 (UserInterface|CreateWidget "/Game/Dropent/Widhget/Win.Win_C"))
      (Variables|Default|SetWinWidget _returnvalue_3))))

(fn ConstructionScript)